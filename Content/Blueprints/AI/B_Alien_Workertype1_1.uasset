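; Alien worker AI that ferries boxes to the truck, scripted as a looping AIMoveTo chain in the event graph.
; Box overlap briefly halts movement and attaches the box to the HoldBox socket.
; Overlapping the player permanently sets EnemyDetected, making it drop any box via floor line trace and flee toward a scatter actor.
; Tick polls the truck's counter; at five, the alien boards by destroying itself and hides the UFO.
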(event `DropBox`
  ;[1 1 1] dropping box
  (`self.Trace floor and dropbox`))

(event `self.ReceiveBeginPlay`
  (bind (_b_truck _b_alien) (`self.Get Truck & Self`))
  ;[1 1 1] Move to objective
  (if (`self.IsCarrying`) :!label _label
    ;[1 1 1] If is carrying box then go to truck
    (bind _returnvalue (`self.If carrying then check if enemy detected or move to truck` :!label _label_2)
      (:`else`
        (`|AIMoveTo` _b_alien (0.0 0.0 0.0) _b_truck
          (:`OnSuccess`
            _)
          (:`OnFail`
            _))
        (if (`self.EnemyDetected`)
          (goto _label_2 :!via `execute2`)
          (else
            (set `self.IsCarrying` false)
            (`KismetSystemLibrary.PrintString` "carrying false")
            (goto _label))))
      (:`then_0`
        ;[1 1 1] Drop box and run away from player
        (`|AIMoveTo` self (`self.Goto Random location`) _returnvalue
          (:`OnSuccess`
            (`KismetSystemLibrary.PrintString` "stop carrying and run away")))))
    (elif (`self.EnemyDetected`)
      (goto _label_2 :!via `execute2`)
      (else
        (bind _returnvalue_2 (`GameplayStatics.GetActorOfClass` (`self.Box type`)))
        (`|AIMoveTo` self (0.0 0.0 0.0) _returnvalue_2
          (:`OnSuccess`
            _)
          (:`OnFail`
            _))
        (`KismetSystemLibrary.Delay` 0.2)
        (goto _label)))))

(event `self.ReceiveTick`
  (params (DeltaSeconds :type "Float (single-precision)"))
  (`self.Are we ready to drive`))

(event `self.Box.OnComponentBeginOverlap`
  (params (OverlappedComponent :type "PrimitiveComponent Object Reference") (OtherActor :type "Actor Object Reference") (OtherComp :type "PrimitiveComponent Object Reference") (OtherBodyIndex :type Integer) (bFromSweep :type Boolean) (SweepResult :type "HitResult Structure (by ref)"))
  ;[1 1 1] On Target Overlap, disable ai movement and wait 1 second
  (cast `/Game/Blueprints/AI/B_Boxes` OtherActor)
  (`self.Deactivate AI Movement`)
  (`KismetSystemLibrary.Delay` 0.2)
  ;[1 1 1] Then pickup object, is now carrying
  (`self.pickup`)
  (set `self.IsCarrying` true)
  (`KismetSystemLibrary.PrintString` "picked up")
  ;[1 1 1] Start movement again
  (`self.Activate AI Movement`))

(event `pickup`
  ;[1 1 1] Pickup box
  (bind _overlappingactors (`self.Check overlapping actor`))
  (for _array_element _overlappingactors
    (if (`self.ActorHasTag` _array_element "Pickup")
      (bind _output_get (set `self.ItemsHolding` _array_element))
      (`self.Carry actor` _output_get (`self.AI`))
      (break))))

(event `self.Box1.OnComponentBeginOverlap`
  (params (OverlappedComponent :type "PrimitiveComponent Object Reference") (OtherActor :type "Actor Object Reference") (OtherComp :type "PrimitiveComponent Object Reference") (OtherBodyIndex :type Integer) (bFromSweep :type Boolean) (SweepResult :type "HitResult Structure (by ref)"))
  ;[1 1 1] If we are overlapping with player, then set condition to true
  (cast `/Game/TwinStickBP/Blueprints/TwinStickPawn` OtherActor)
  (set `self.EnemyDetected` true)
  (if (`self.EnemyDetected`)
    (`KismetSystemLibrary.PrintString` "Saw player, stop movement")))

(event `Are we ready to drive`
  ;[1 1 1] Check with truck if we are ready to hop into truck
  (bind _returnvalue (`GameplayStatics.GetActorOfClass` "/Game/Blueprints/AI/B_Truck.B_Truck_C"))
  (if (== (`/Game/Blueprints/AI/B_Truck.Counter` _returnvalue) 5)
    (`|ExecutionSequence`
      (:`then_0`
        (`self.Jump into truck`))
      (:`then_1`
        (`SceneComponent.ToggleVisibility` (`/Game/Blueprints/AI/B_Truck.AlienUfo` _returnvalue) false)))))

(event `Jump into truck`
  (bind (_b_truck _b_alien) (`self.Get Truck & Self`))
  ;[1 1 1] Jump into truck by destroying actor
  (`|AIMoveTo` _b_alien (0.0 0.0 0.0) _b_truck 10.0
    (:`OnSuccess`
      _)
    (:`OnFail`
      _))
  (`KismetSystemLibrary.PrintString` "Loading ai into truck")
  (`KismetSystemLibrary.Delay` 2.0)
  (`self.K2_DestroyActor`))

(fn `Activate AI Movement`
  (`ActorComponent.Activate` (`self.CharacterMovement`) false))

(fn `Carry actor`
  (params (Box :type "Actor Object Reference") (Alien :type "SceneComponent Object Reference"))
  (`self.K2_AttachToComponent` Box Alien "HoldBox" "SnapToTarget" "KeepWorld" "KeepWorld" true)
  (set `self.IsCarrying` true))

(fn `Check overlapping actor`
  (returns (OverlappingActors :type "Array of Actor Object Reference"))
  (if (not (`self.IsCarrying`))
    (return (`self.GetOverlappingActors` (`self.Box type`)))))

(fn `Deactivate AI Movement`
  (bind _charactermovement (`self.CharacterMovement`))
  (`MovementComponent.StopMovementImmediately` _charactermovement)
  (`ActorComponent.Deactivate` _charactermovement))

(fn `Destroy Box`
  (params (Truck :type "Actor Object Reference"))
  (bind _returnvalue (`GameplayStatics.GetActorOfClass` (`self.Box type`)))
  (if (`self.IsOverlappingActor` _returnvalue Truck)
    (`self.K2_DestroyActor` _returnvalue)))

(fn `Detach and give new transform`
  (params (`New Transform` :type "Vector Structure"))
  (bind _itemsholding (`self.ItemsHolding`))
  (`self.K2_DetachFromActor` _itemsholding "KeepWorld" "KeepWorld" "KeepWorld")
  (`self.K2_SetActorTransform` _itemsholding (`KismetMathLibrary.MakeTransform` `New Transform` (`KismetMathLibrary.RandomRotator` true) (0.5 0.5 0.5)) false false))

(fn `Get Truck & Self`
  (returns (B_Truck :type "/Game/Blueprints/AI/B_Truck Object Reference") (B_Alien :type "Self Object Reference"))
  (bind _returnvalue (`GameplayStatics.GetActorOfClass` "/Game/Blueprints/AI/B_Truck.B_Truck_C"))
  (return _returnvalue self))

(fn `Reset, Find another box`
  (if (`self.IsCarrying`)
    _))

(fn `Trace floor and dropbox`
  (bind (_player_location _floor_location) (`self.From Pickup to floor level`))
  (if (`self.EnemyDetected`)
    (bind (_outhit _returnvalue) (`KismetSystemLibrary.LineTraceSingle` _player_location _floor_location "TraceTypeQuery1"))
    (if _returnvalue
      (`self.Detach and give new transform` (`.Location` (`GameplayStatics.BreakHitResult` _outhit)))
      (set `self.IsCarrying` false))))

(fn `UserConstructionScript`)