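; B_Truck is a truck that shows cargo as boxes reach its pickup collision and drives off along timelines.
; Each B_Boxes or B_Boxes2 overlap reveals a random, possibly already visible, box mesh, increments a counter and restarts a two-minute timer.
; When the timer expires with the counter at exactly five, a timeline moves the truck.
; Separately, a TwinStickPawn overlapping the player detector starts a second movement timeline after a delay.
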(event `self.ReceiveBeginPlay`
  ;[1 1 1] Set inventory, boxes and ai mesh visibility to false on begin play
  (set `self.Counter` 0)
  (`SceneComponent.SetVisibility` (`self.Box Array`) false false)
  (`SceneComponent.SetVisibility` (`self.AI Mesh Array`) false false))

(event `self.PickupCollision.OnComponentBeginOverlap`
  (params (OverlappedComponent :type "PrimitiveComponent Object Reference") (OtherActor :type "Actor Object Reference") (OtherComp :type "PrimitiveComponent Object Reference") (OtherBodyIndex :type Integer) (bFromSweep :type Boolean) (SweepResult :type "HitResult Structure (by ref)"))
  ;[1 1 1] Check collision with boxes, toggle visibility and start a timer on first visibility toggle
  (`|ExecutionSequence`
    (:`then_0`
      (if true
        (cast `/Game/Blueprints/AI/B_Boxes` OtherActor)
        (`self.Toggle visiblity` :!label _label)
        (`/Engine/EditorBlueprintResources/StandardMacros.IncrementInt` (`self.Counter`)
          (:`  `
            (if true
              (`KismetSystemLibrary.K2_SetTimerDelegate` (delegate `Load players into trucks and drive`) 120.0))))))
    (:`then_1`
      (if true
        (cast `/Game/Blueprints/AI/B_Boxes2` OtherActor)
        (goto _label)))))

(event `Toggle visiblity`
  ;[1 1 1] Random box visibility on collision
  (`SceneComponent.SetVisibility` (`KismetArrayLibrary.Array_Random` (`self.Box Array`)) true false)
  (`KismetSystemLibrary.PrintString` "Toggling"))

(event `Load players into trucks and drive`
  ;[1 1 1] After timer ends check if inventory load meets condition
  (if (== (`self.Counter`) 5)
    (`KismetSystemLibrary.PrintString` "Load players into trucks and drive")
    (`self.If Full Start Driving`)))

(event `If Full Start Driving`
  ;[1 1 1] If all boxes loaded, drive
  (`KismetSystemLibrary.Delay` 1.0)
  (`KismetSystemLibrary.PrintString` "All Boxes Loaded")
  (`self.Truck Full Animation`)
  (`KismetSystemLibrary.PrintString` "Start Driving"))

(event `Truck Full Animation`
  (bind _maintruck (`self.MainTruck`))
  ;[1 1 1] Move on X axis
  (bind (_direction _newtrack_0) (`Timeline|Timeline_0`)
    (:`Update`
      (`SceneComponent.K2_SetWorldLocation` _maintruck (+ _newtrack_0 (`SceneComponent.K2_GetComponentLocation` _maintruck)) false false))))

(event `Start truck if overlap with player`
  (bind _maintruck (`self.MainTruck`))
  ;[1 1 1] Move on X axis on player overlap
  (bind (_direction _newtrack_0) (`Timeline|Timeline_1`)
    (:`Update`
      (`SceneComponent.K2_SetWorldLocation` _maintruck (+ _newtrack_0 (`SceneComponent.K2_GetComponentLocation` _maintruck)) false false))))

(event `self.Player detector.OnComponentBeginOverlap`
  (params (OverlappedComponent :type "PrimitiveComponent Object Reference") (OtherActor :type "Actor Object Reference") (OtherComp :type "PrimitiveComponent Object Reference") (OtherBodyIndex :type Integer) (bFromSweep :type Boolean) (SweepResult :type "HitResult Structure (by ref)"))
  ;[1 1 1] starting truck when overlap with player
  (cast `/Game/TwinStickBP/Blueprints/TwinStickPawn` OtherActor)
  (`KismetSystemLibrary.PrintString` "player truck overlap")
  (`KismetSystemLibrary.Delay` 15.0)
  (`self.Start truck if overlap with player`))

(fn `AI Mesh Array`
  (returns (Array :type "Array of StaticMeshComponent Object Reference"))
  (return (`|MakeArray` (`self.AlienUfo`) (`self.AlienUfo1`))))

(fn `Box Array`
  (returns (Array :type "Array of StaticMeshComponent Object Reference"))
  (return (`|MakeArray` (`self.Box7`) (`self.Box2`) (`self.Box3`) (`self.Box4`) (`self.Box5`) (`self.Box6`) (`self.Box1`) (`self.Box8`) (`self.Box9`) (`self.Box10`) (`self.Box11`) (`self.Box12`))))

(fn `Check visibility true`
  (if (`SceneComponent.IsVisible` (`self.Box7`))
    (if (`SceneComponent.IsVisible` (`self.Box2`))
      (if (`SceneComponent.IsVisible` (`self.Box3`))
        (if (`SceneComponent.IsVisible` (`self.Box4`))
          (if (`SceneComponent.IsVisible` (`self.Box5`))
            (if (`SceneComponent.IsVisible` (`self.Box6`))
              (if (`SceneComponent.IsVisible` (`self.Box1`))
                (if (`SceneComponent.IsVisible` (`self.Box8`))
                  (if (`SceneComponent.IsVisible` (`self.Box9`))
                    (if (`SceneComponent.IsVisible` (`self.Box10`))
                      (if (`SceneComponent.IsVisible` (`self.Box11`))
                        (if (`SceneComponent.IsVisible` (`self.Box12`))
                          (return))))))))))))))

(fn `UserConstructionScript`)